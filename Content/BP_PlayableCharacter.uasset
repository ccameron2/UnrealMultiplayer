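; BP_PlayableCharacter is a playable character Blueprint that carries a floating name label showing its identity and network role.
; On BeginPlay it casts the NameDetails component's widget to BP_NameDetails and fills it with the actor's display name and local role.
; Every Tick it rotates the label in world space to face player 0's camera, billboard style.
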(event `self.ReceiveBeginPlay`
  (bind _asbp_name_details (cast `/Game/BP_NameDetails` (`WidgetComponent.GetUserWidgetObject` (`self.NameDetails`))))
  (set `/Game/BP_NameDetails.Actor Name` (`KismetSystemLibrary.GetDisplayName` self) _asbp_name_details)
  (set `/Game/BP_NameDetails.Actor Role` (`|GetEnumeratorNameAsString` (`self.GetLocalRole` self)) _asbp_name_details))

(event `self.ReceiveTick`
  (params (DeltaSeconds :type "Float (single-precision)"))
  (`SceneComponent.K2_SetWorldRotation` (`self.NameDetails`) (`KismetMathLibrary.FindLookAtRotation` (`SceneComponent.K2_GetComponentLocation` (`self.NameDetails`)) (`PlayerCameraManager.GetCameraLocation` (`GameplayStatics.GetPlayerCameraManager` 0))) false false))

(fn `UserConstructionScript`)